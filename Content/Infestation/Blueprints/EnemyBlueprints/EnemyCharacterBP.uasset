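; Base enemy character Blueprint for Infestation that handles death when its health runs out.
; On BeginPlay it binds to the HealthComponent's damage event, and at zero health a QueenBP instance runs its own KillQueen logic.
; Other enemies notify their assigned spawner of the despawn, fire the game state's enemy death delegate, then destroy themselves.
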(event `self.ReceiveTick`
  (params (DeltaSeconds :type "Float (single-precision)")))

(event `self.ReceiveBeginPlay`
  (add `/Game/Infestation/Blueprints/HealthComponent.HandleTakeDamage` (`self.HealthComponent`) (delegate `OnEnemyHealthChanged`)))

(event `OnEnemyHealthChanged`
  (params (DamageActor :type "/Game/Infestation/Blueprints/HealthComponent Object Reference") (Health :type "Float (double-precision)") (Damage :type "Float (double-precision)") (DamageType :type "DamageType Object Reference") (InstigatedBy :type "Controller Object Reference") (DamageCauser :type "Actor Object Reference"))
  (bind _enemyspawner (`self.enemySpawner`))
  (if (<= Health 0.0)
    (bind _asqueen_bp (cast `/Game/Infestation/Blueprints/EnemyBlueprints/QueenBP` self)
      (:`then`
        (`/Game/Infestation/Blueprints/EnemyBlueprints/QueenBP.KillQueen` _asqueen_bp))
      (:`CastFailed`
        (if (`KismetSystemLibrary.IsValid` _enemyspawner)
          (`EnemySpawner.HandleEnemyDespawn` _enemyspawner))
        (bind _asinfestation_game_state (cast `InfestationGameState` (`GameplayStatics.GetGameState`)))
        (`InfestationDelegates.onEnemyDeathDelegate` (`InfestationGameState.delegates` _asinfestation_game_state) self)
        (`self.K2_DestroyActor`)))))

(fn `SetEnemySpawner`
  (params (spawner :type "/Game/Infestation/Blueprints/EnemySpawnerBP Object Reference"))
  (set `self.enemySpawner` spawner))

(fn `UserConstructionScript`)