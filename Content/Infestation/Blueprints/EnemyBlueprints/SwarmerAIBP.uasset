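; AI controller for the Swarmer enemy, handling objective generation and target acquisition.
; A looping timer started on BeginPlay periodically updates the objective generators through ObjectiveGenerationComp.
; While it has no valid target, a perception update that successfully senses a valid attack target locks it in.
; The find is then broadcast through the InfestationGameState target-found delegate and passed on to alert local enemies.
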(event `self.ReceiveBeginPlay`
  (`KismetSystemLibrary.K2_SetTimerDelegate` (delegate `UpdateGenerators`) (`AIObjectiveGenerationComponent.generatorsUpdateTimer` (`self.objectiveGenerationComp`)) true))

(event `UpdateGenerators`
  (`AIObjectiveGenerationComponent.UpdateGenerators` (`self.objectiveGenerationComp`)))

(event `self.perceptionComp.OnTargetPerceptionUpdated`
  (params (Actor :type "Actor Object Reference") (Stimulus :type "AIStimulus Structure"))
  (bind _targetactor (`self.targetActor`))
  (if (not (`KismetSystemLibrary.IsValid` (`self.targetActor`)))
    (bind _returnvalue (`self.ValidAttackTarget` Actor))
    (if _returnvalue
      (bind _returnvalue_2 (`self.WasSuccussfullySensed` Stimulus))
      (if _returnvalue_2
        (`self.SetAttackTarget` Actor)
        (bind _asinfestation_game_state (cast `InfestationGameState` (`GameplayStatics.GetGameState`)))
        (`InfestationDelegates.onTargetFoundDelegate` (`InfestationGameState.delegates` _asinfestation_game_state) (`self.K2_GetPawn` self) _targetactor)
        (`self.AlertLocalEnemies` _targetactor)))))

(fn `UserConstructionScript`)