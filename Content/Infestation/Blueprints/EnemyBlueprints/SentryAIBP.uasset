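; SentryAIBP is the AI Blueprint for the Sentry enemy, choosing which behavior it runs.
; A looping timer updates objective generators, feeds their objectives to the behavior selector, then runs and records any returned option.
; Tick polls whether the behavior tree is still running; when it is not, it starts cooldowns for that behavior and its parent groups, reselects immediately and resets the timer.
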(event `self.ReceiveBeginPlay`
  (`KismetSystemLibrary.K2_SetTimerDelegate` (delegate `Run New Behavior`) (`self.runNewBehaviorTimer`) true))

(event `Run New Behavior`
  (bind _objectivegenerationcomp (`self.objectiveGenerationComp`))
  (`AIObjectiveGenerationComponent.UpdateGenerators` _objectivegenerationcomp)
  (bind _returnvalue (`AIObjectiveGenerationComponent.GetGeneratedObjectives` _objectivegenerationcomp))
  (bind _returnvalue_2 (`AIBehaviorSelectorComponent.SelectBehavior` (`self.behaviorSelectorComp`) _returnvalue (`BrainComponent.IsRunning` (`self.behaviorComp`))))
  (if (not (== (`.behavior` (break `AIBehaviorOption` _returnvalue_2)) null))
    (`self.RunBehaviorOption` _returnvalue_2)
    (set `AIBehaviorSelectorComponent.currentBehaviorOption` _returnvalue_2 (`self.behaviorSelectorComp`))))

(event `self.ReceiveTick`
  (params (DeltaSeconds :type "Float (single-precision)"))
  (bind _behaviorselectorcomp (`self.behaviorSelectorComp`))
  ;[1 1 1] Only way to check if the behavior tree is still running. If it has finished or stopped, start the finished behavior's cooldown and call Run New Behavior.
  (if (not (`BrainComponent.IsRunning` (`self.behaviorComp`)))
    (`AIBehaviorSelectorComponent.StartCooldownForBehaviorAndParentGroups` _behaviorselectorcomp (`AIBehaviorSelectorComponent.currentBehaviorOption` _behaviorselectorcomp))
    (`self.Run New Behavior`)
    ;[1 1 1] Can only have one timer for each event of an actor. So to reset it, we can just call the function again.
    (`KismetSystemLibrary.K2_SetTimerDelegate` :`Time` (`self.runNewBehaviorTimer`) :`bLooping` true)))

(fn `UserConstructionScript`)