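; Hitscan gun weapon that fires instant ray traces and damages enemy characters it hits.
; UseWeapon checks the attack cooldown and clip ammo, consumes ammo, traces once per pellet via ShootRay, then resets the cooldown.
; Enemy hits apply per-pellet damage and post a temporary damage message to the player's log.
; Shots are visualized with debug arrows from the muzzle position to the impact point.
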(event `self.UseWeapon`
  (params (actor :type "Actor Object Reference"))
  (bind _ammoconsumedpershot (`self.ammoConsumedPerShot`))
  ;[1 1 1] Checks for ammo and consumes it, before checking to see what the bullet hit and damaging it if it was an enemy
  (bind _returnvalue (`self.CanAttack`))
  (if _returnvalue
    (bind _returnvalue_2 (`self.GetAmmoInClip`))
    (if (>= _returnvalue_2 _ammoconsumedpershot)
      (`self.ConsumeAmmo` _ammoconsumedpershot)
      (for _ (range 1 (+ (`self.pelletsPerShot`) 1))
        (bind _returnvalue_3 (`self.ShootRay` actor 100000.0))
        (bind (_bblockinghit _binitialoverlap _time _distance _location _impactpoint _normal _impactnormal _physmat _hitactor) (`GameplayStatics.BreakHitResult` _returnvalue_3))
        (bind _asenemy_character_bp (cast `/Game/Infestation/Blueprints/EnemyBlueprints/EnemyCharacterBP` _hitactor)
          (:`then`
            (bind _returnvalue_4 (`GameplayStatics.ApplyDamage` _asenemy_character_bp (`KismetMathLibrary.Conv_IntToDouble` (`self.damagePerHit`))))
            ;;[1 1 1] Displays a message showing the player hit an enemy (Temp)
            (bind _asmy_player_character (cast `MyPlayerCharacter` actor))
            (`MessageLogComponent.AddMessage` (`MyPlayerCharacter.messageLog` _asmy_player_character) (`KismetTextLibrary.Conv_StringToText` (`KismetStringLibrary.BuildString_Double` "" "" _returnvalue_4 " damage dealt!"))))
          (:`CastFailed`
            _))
        (`self.DrawBulletLine` _impactpoint))
      (`self.ResetAttackCooldown`))))

(event `DrawBulletLine`
  (params (hitPoint :type "Vector Structure"))
  (`KismetSystemLibrary.DrawDebugArrow` (`SceneComponent.K2_GetComponentLocation` (`self.shotPosition`)) hitPoint 1.0 (struct :`R` 1.0 :`A` 1.0) 1.0 1.0))

(event `self.StopUsingWeapon`)

(fn `UserConstructionScript`)