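; AI objective generator that turns nearby attack targets into melee target opportunities for an AI's combat objective.
; On each update it queries actors of the configured types within a search radius around the controlled pawn, falling back to the perception component's owner with a warning.
; It then rebuilds the melee objective's opportunity list, flagging whether each target is currently seen by sight perception, or clears it when none are found.
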(event `self.OnUpdate`
  (bind _attacktargets (`self.FindValidAttackTargets`))
  (bind _output_get (set `self.attackTargets` _attacktargets))
  (if (`KismetArrayLibrary.Array_IsEmpty` _output_get)
    (bind _returnvalue (`self.GetExistingObjective` "/Script/ProjectInfestation.AIObjective_MeleeTarget"))
    (bind _asaiobjective_melee_target (cast `AIObjective_MeleeTarget` _returnvalue))
    (`KismetArrayLibrary.Array_Clear` (`AIObjective_MeleeTarget.meleeTargetOpportunities` _asaiobjective_melee_target))
    (else
      (bind _returnvalue_2 (`self.GetOrCreateObjective` "/Script/ProjectInfestation.AIObjective_MeleeTarget"))
      (bind _asaiobjective_melee_target_2 (cast `AIObjective_MeleeTarget` _returnvalue_2))
      (`KismetArrayLibrary.Array_Clear` (`AIObjective_MeleeTarget.meleeTargetOpportunities` _asaiobjective_melee_target_2))
      (for _array_element (`self.attackTargets`)
        (bind _meleeattackopportunity (`self.CreateMeleeAttackOpportunity` _array_element))
        (`KismetArrayLibrary.Array_Add` (`AIObjective_MeleeTarget.meleeTargetOpportunities` _asaiobjective_melee_target_2) _meleeattackopportunity))
      (`KismetSystemLibrary.PrintString` null "Melee Target Opportunities Generated"))))

(fn `CreateMeleeAttackOpportunity`
  (params (MeleeTarget :type "Actor Object Reference"))
  (returns (MeleeAttackOpportunity :type "UAIOpportunity_MeleeTarget Structure"))
  (for _array_element (`AIPerceptionComponent.GetCurrentlyPerceivedActors` (`self.ownerPerceptionComponent`) "/Script/AIModule.AISense_Sight")
    ;[1 1 1] Melee target is in sight
    (if (== _array_element MeleeTarget)
      (return (make `UAIOpportunity_MeleeTarget` MeleeTarget true))))
  ;[1 1 1] Melee target isn't in sight
  (return (make `UAIOpportunity_MeleeTarget` MeleeTarget)))

(fn `FindValidAttackTargets`
  (returns (AttackTargets :type "Array of Actor Object Reference"))
  (locals (WarningMsg :type String :default "CombatAIObjectiveGeneration FindValidAttackTargets(): Warning, OwnerPerceptionComponent is on a pawn not a controller."))
  (bind _attacktargettypes (`self.attackTargetTypes`))
  (bind _searchradius (`self.searchRadius`))
  (bind _returnvalue (`ActorComponent.GetOwner` (`self.ownerPerceptionComponent`)))
  (bind _asaicontroller (cast `AIController` _returnvalue)
    (:`then`
      (bind _returnvalue_2 (`InfestationUtilities.QuerySurroundingActors` :`originActor` (`Controller.K2_GetPawn` _asaicontroller) :`radius` _searchradius :`objectTypes` _attacktargettypes :`drawTime` 0.1))
      (return _returnvalue_2))
    (:`CastFailed`
      (`KismetSystemLibrary.PrintString` null (`local.WarningMsg`))
      (bind _returnvalue_3 (`InfestationUtilities.QuerySurroundingActors` :`originActor` _returnvalue :`radius` _searchradius :`objectTypes` _attacktargettypes :`drawTime` 0.1))
      (return _returnvalue_3))))