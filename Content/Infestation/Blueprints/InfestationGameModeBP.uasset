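; Game mode Blueprint for Infestation that handles the win, lose and pause screens.
; WinGame and LoseGame each show their end screen with UI-only input and a mouse cursor, pause the game, and set GameEnded.
; PauseGame and UnpauseGame add or remove the pause widget and switch input mode, cursor and paused state.
; GameEnded blocks pausing and unpausing once the match is over.
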(event `self.WinGame`
  (bind _returnvalue (`GameplayStatics.GetPlayerController` 0))
  (bind _returnvalue_2 (`|CreateWidget` "/Game/Infestation/Widgets/VictoryScreen.VictoryScreen_C"))
  (`UserWidget.AddToViewport` _returnvalue_2 1)
  (`Widget.SetKeyboardFocus` _returnvalue_2)
  (set `PlayerController.bShowMouseCursor` true _returnvalue)
  (`WidgetBlueprintLibrary.SetInputMode_UIOnlyEx` _returnvalue _returnvalue_2)
  (`GameplayStatics.SetGamePaused` true)
  (set `self.gameEnded` true :!label _label))

(event `self.LoseGame`
  (bind _returnvalue (`GameplayStatics.GetPlayerController` 0))
  (bind _returnvalue_2 (`|CreateWidget` "/Game/Infestation/Widgets/GameOverScreen.GameOverScreen_C"))
  (`UserWidget.AddToViewport` _returnvalue_2 1)
  (`Widget.SetKeyboardFocus` _returnvalue_2)
  (set `PlayerController.bShowMouseCursor` true _returnvalue)
  (`WidgetBlueprintLibrary.SetInputMode_UIOnlyEx` _returnvalue _returnvalue_2)
  (`GameplayStatics.SetGamePaused` true)
  (goto _label))

(event `self.PauseGame`
  (bind _returnvalue (`GameplayStatics.GetPlayerController` 0))
  (if (not (`self.gameEnded`))
    (bind _returnvalue_2 (`|CreateWidget` "/Game/Infestation/Widgets/PauseScreen.PauseScreen_C"))
    (`UserWidget.AddToViewport` _returnvalue_2 1)
    (`Widget.SetKeyboardFocus` _returnvalue_2)
    (set `PlayerController.bShowMouseCursor` true _returnvalue)
    (`WidgetBlueprintLibrary.SetInputMode_GameAndUIEx` _returnvalue _returnvalue_2)
    (`GameplayStatics.SetGamePaused` true)))

(event `self.UnpauseGame`
  (bind _returnvalue (`GameplayStatics.GetPlayerController` 0))
  (if (not (`self.gameEnded`))
    (bind _foundwidgets (`WidgetBlueprintLibrary.GetAllWidgetsOfClass` "/Game/Infestation/Widgets/PauseScreen.PauseScreen_C"))
    (`Widget.RemoveFromParent` _foundwidgets)
    (`WidgetBlueprintLibrary.SetInputMode_GameOnly` _returnvalue)
    (set `PlayerController.bShowMouseCursor` false _returnvalue)
    (`GameplayStatics.SetGamePaused` false)))

(fn `UserConstructionScript`)