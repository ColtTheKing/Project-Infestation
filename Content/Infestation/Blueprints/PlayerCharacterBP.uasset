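; Player character Blueprint for Infestation that links its weapon arsenal, health component and UI.
; BeginPlay creates the HUD and a hidden weapon wheel; opening it shows the cursor, and closing selects the weapon under the mouse.
; Selections return via a GameState delegate to activate the arsenal slot, while Tick refreshes the wheel once through a dirty flag.
; Death triggers the GameMode's LoseGame; upgrade functions raise max health or weapon damage and log messages.
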(event `onWeaponWheelSelectDelegate_Event`
  (params (weaponInd :type Integer))
  (bind _weaponarsenal (`self.weaponArsenal`))
  (bind _returnvalue (`ArsenalComponent.GetWeaponAtIndex` _weaponarsenal weaponInd))
  (`KismetSystemLibrary.PrintString` (`KismetStringLibrary.Concat_StrStr` "SWAPPED TO " (`KismetStringLibrary.Conv_NameToString` (`Weapon.weaponName` _returnvalue))) true true (struct :`G` 0.66 :`B` 1.0 :`A` 1.0) 10.0)
  (`ArsenalComponent.ActivateIndex` _weaponarsenal weaponInd))

(event `self.ReceiveBeginPlay`
  (bind _asinfestation_game_state (cast `InfestationGameState` (`GameplayStatics.GetGameState`)))
  (add `InfestationDelegates.onWeaponWheelSelectDelegate` (`InfestationGameState.delegates` _asinfestation_game_state) (delegate `onWeaponWheelSelectDelegate_Event`))
  (bind _returnvalue (`|CreateWidget` "/Game/Infestation/Widgets/UserInterface.UserInterface_C"))
  (`UserWidget.AddToViewport` _returnvalue 0)
  (bind _returnvalue_2 (`|CreateWidget` "/Game/Infestation/Widgets/WeaponWheelScreen.WeaponWheelScreen_C"))
  (`Widget.SetVisibility` _returnvalue_2 "Hidden")
  (`UserWidget.AddToViewport` _returnvalue_2 0)
  (set `self.WeaponWheel` _returnvalue_2)
  (`WidgetBlueprintLibrary.SetInputMode_GameOnly` (`GameplayStatics.GetPlayerController` 0))
  (add `/Game/Infestation/Blueprints/HealthComponent.HandleTakeDamage` (`self.HealthComponent`) (delegate `CustomEvent`))
  (set `self.ArsenalNeedsUpdate` true))

(event `CustomEvent`
  (params (DamageActor :type "/Game/Infestation/Blueprints/HealthComponent Object Reference") (Health :type "Float (double-precision)") (Damage :type "Float (double-precision)") (DamageType :type "DamageType Object Reference") (InstigatedBy :type "Controller Object Reference") (DamageCauser :type "Actor Object Reference"))
  (if (<= Health 0.0)
    (bind _asinfestation_game_mode_bp (cast `/Game/Infestation/Blueprints/InfestationGameModeBP` (`GameplayStatics.GetGameMode`)))
    (`InfestationGameMode.LoseGame` _asinfestation_game_mode_bp)))

(event `self.ReceiveTick`
  (params (DeltaSeconds :type "Float (single-precision)"))
  (if (`self.ArsenalNeedsUpdate`)
    (`/Game/Infestation/Widgets/WeaponWheelScreen.UpdatePlayerArsenal` (`self.WeaponWheel`) (`self.weaponArsenal`))
    (set `self.ArsenalNeedsUpdate` false)))

(event `self.OpenWeaponWheel`
  (bind _returnvalue (`GameplayStatics.GetPlayerController` 0))
  (`WidgetBlueprintLibrary.SetInputMode_GameAndUIEx` _returnvalue (`self.WeaponWheel`))
  (set `PlayerController.bShowMouseCursor` true _returnvalue)
  (`Widget.SetVisibility` (`self.WeaponWheel`) "Visible")
  (set `self.WeaponWheelOpen` true))

(event `self.CloseWeaponWheel`
  (bind _returnvalue (`GameplayStatics.GetPlayerController` 0))
  (`/Game/Infestation/Widgets/WeaponWheelScreen.SelectWeaponAtMousePos` (`self.WeaponWheel`))
  (`WidgetBlueprintLibrary.SetInputMode_GameOnly` _returnvalue)
  (set `PlayerController.bShowMouseCursor` false _returnvalue)
  (`Widget.SetVisibility` (`self.WeaponWheel`) "Hidden")
  (set `self.WeaponWheelOpen` false))

(fn `Increase Armour`
  (params (amount :type Integer))
  (bind _healthcomponent (`self.HealthComponent`))
  (`/Game/Infestation/Blueprints/HealthComponent.Set Max Health` _healthcomponent (+ (`/Game/Infestation/Blueprints/HealthComponent.MaxHealth` _healthcomponent) amount))
  (`MessageLogComponent.AddMessage` (`self.messageLog`) (`KismetTextLibrary.Conv_StringToText` (`KismetStringLibrary.BuildString_Int` "" "Max HP: " (`/Game/Infestation/Blueprints/HealthComponent.MaxHealth` _healthcomponent)))))

(fn `Upgrade Weapon`
  (params (`Gun Type` :type Name) (`Damage Mult` :type "Float (double-precision)"))
  (bind _returnvalue (`ArsenalComponent.GetWeaponOfType` (`self.weaponArsenal`) `Gun Type`))
  (if (`KismetSystemLibrary.IsValid` _returnvalue)
    (`Weapon.ModifyDamagePerHit` _returnvalue `Damage Mult`)
    (`MessageLogComponent.AddMessage` (`self.messageLog`) (`KismetTextLibrary.Conv_StringToText` (`KismetStringLibrary.BuildString_Double` "" "Damage increased by " `Damage Mult` "X")))))

(fn `UserConstructionScript`)