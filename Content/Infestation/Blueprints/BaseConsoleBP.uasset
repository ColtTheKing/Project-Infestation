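; Interactive console that diverts power away from its linked enemy spawner, shutting it down and rewarding the player.
; Interact starts a looping one-second timer on DiversionSequence if the spawner is valid, counting down with periodic "seconds left" posts to the player's message log.
; At zero it destroys the spawner and TriggerUpgrade grants a random option, either armour or pistol damage.
; The looping timer is never cleared here.
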(event `self.Interact`
  (if (`KismetSystemLibrary.IsValid` (`self.baseSpawner`))
    (`KismetSystemLibrary.K2_SetTimer` null "DiversionSequence" 1.0 true)))

(fn `DiversionSequence`
  (bind _result (`/Engine/EditorBlueprintResources/StandardMacros.DecrementInt` (`self.sequenceDuration`))
    (:`  `
      (if (== _result 0)
        (`self.K2_DestroyActor` (`self.baseSpawner`))
        (`self.TriggerUpgrade`)
        (elif (== (mod _result 5) 0)
          (bind _asplayer_character_bp (cast `/Game/Infestation/Blueprints/PlayerCharacterBP` (`GameplayStatics.GetPlayerCharacter` 0)))
          (`MessageLogComponent.AddMessage` (`MyPlayerCharacter.messageLog` _asplayer_character_bp) (`KismetTextLibrary.Conv_StringToText` (`KismetStringLibrary.BuildString_Int` "" "" _result " seconds left"))))))))

(fn `TriggerUpgrade`
  (locals (randomOption :type String))
  (bind _upgradeoptions (`self.upgradeOptions`))
  (bind _asplayer_character_bp (cast `/Game/Infestation/Blueprints/PlayerCharacterBP` (`GameplayStatics.GetPlayerCharacter` 0)))
  (bind _messagelog (`MyPlayerCharacter.messageLog` _asplayer_character_bp))
  (`MessageLogComponent.AddMessage` _messagelog "Power diverted! Enemies will no longer spawn here")
  (bind _output_get (set `local.randomOption` (`|GetArrayItem` _upgradeoptions (`KismetMathLibrary.RandomInteger` (`KismetArrayLibrary.Array_Length` _upgradeoptions)))))
  (switch `string` _output_get
    (:`Fortified Armour`
      (`/Game/Infestation/Blueprints/PlayerCharacterBP.Increase Armour` _asplayer_character_bp 25)
      (bind _returnvalue (`KismetTextLibrary.Conv_StringToText` _output_get))
      (`MessageLogComponent.AddMessage` _messagelog _returnvalue))
    (:`Pistol Damage Boost`
      (`/Game/Infestation/Blueprints/PlayerCharacterBP.Upgrade Weapon` _asplayer_character_bp "Pistol" 5.0)
      (`MessageLogComponent.AddMessage` _messagelog _returnvalue))))

(fn `UserConstructionScript`)