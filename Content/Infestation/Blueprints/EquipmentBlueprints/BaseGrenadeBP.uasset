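; Base grenade actor that explodes on a timer started at BeginPlay.
; When the timer fires, it spawns GrenadeExplosionBP at the grenade mesh's transform and destroys itself.
; It also loops over EnemyCharacter actors overlapping its AreaOfEffect, but the cast leads to no action and the Damage variable is unused, so it deals no damage itself.
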(event `self.ReceiveBeginPlay`
  (`KismetSystemLibrary.K2_SetTimerDelegate` (delegate `Detonate`) (`self.detonationTimer`)))

(event `Detonate`
  (`|SpawnActorFromClass` "/Game/Infestation/Blueprints/EffectBlueprints/GrenadeExplosionBP.GrenadeExplosionBP_C" (`SceneComponent.K2_GetComponentToWorld` (`self.GrenadeMesh`)) "Undefined" "OverrideRootScale" null null)
  (for _array_element (`PrimitiveComponent.GetOverlappingActors` (`self.AreaOfEffect`) "/Script/ProjectInfestation.EnemyCharacter")
    (cast `EnemyCharacter` _array_element))
  (`self.K2_DestroyActor`))

(fn `UserConstructionScript`)